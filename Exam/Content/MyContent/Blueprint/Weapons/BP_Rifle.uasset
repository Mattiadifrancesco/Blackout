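; Rifle weapon Blueprint that provides automatic hitscan fire for the player's survivor character.
; StartFire caches the character and starts a looping timer at FireRate, which StopFire clears.
; Each shot consumes ammo, then, if any remains, plays a montage and line-traces from the follow camera within a random spread cone.
; Hits apply base damage and spawn an emitter, and traces are debug-drawn.
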(event `self.StartFire`
  (bind _asbp_survivor_character (cast `/Game/MyContent/Blueprint/Character/BP_Survivor_Character` (`GameplayStatics.GetPlayerCharacter` 0)))
  (bind _returnvalue (`KismetSystemLibrary.K2_SetTimerDelegate` (delegate `ShootRifleBullet`) (`self.FireRate`) true))
  (set `self.FireTimerHandle` _returnvalue))

(event `ShootRifleBullet`
  (`self.ConsumeAmmo`)
  (if (not (<= (`self.CurrentAmmo`) 0))
    (`self.PlayAnimMontage`)
    (bind _followcamera (`/Game/MyContent/Blueprint/Character/BP_Survivor_Character.FollowCamera` (stale `self.StartFire` _asbp_survivor_character)))
    (bind _returnvalue (`SceneComponent.K2_GetComponentLocation` _followcamera))
    (bind (_outhit _returnvalue_2) (`KismetSystemLibrary.LineTraceSingle` :`Start` _returnvalue :`End` (+ _returnvalue (* (`KismetMathLibrary.RandomUnitVectorInConeInDegrees` (`SceneComponent.GetForwardVector` _followcamera) (`self.SpreadAngle`)) 10000.0)) :`TraceChannel` "TraceTypeQuery2" :`DrawDebugType` "ForDuration"))
    (if _returnvalue_2
      (`GameplayStatics.ApplyDamage` (`.HitActor` (`GameplayStatics.BreakHitResult` _outhit)) (`self.BaseDMG`))
      (`GameplayStatics.SpawnEmitterAtLocation` null))))

(event `self.StopFire`
  (`KismetSystemLibrary.K2_ClearAndInvalidateTimerHandle` (`self.FireTimerHandle`)))

(fn `UserConstructionScript`
  (`parent.UserConstructionScript`))