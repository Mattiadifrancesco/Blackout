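; Base weapon Blueprint for the survivor character, picked up by walking into its sphere trigger.
; On overlap it disables the sphere, attaches the weapon mesh to the right-hand socket and registers itself as the character's current weapon and type.
; Fire and attack events are empty stubs, presumably for child weapons, alongside a montage helper.
; Consuming ammo down to zero stops firing, clears the character's weapon and destroys the actor.
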(event `self.ReceiveBeginPlay`
  (bind _asbp_survivor_character (cast `/Game/MyContent/Blueprint/Character/BP_Survivor_Character` (`GameplayStatics.GetPlayerCharacter` 0)))
  (set `self.CharacterRef` _asbp_survivor_character)
  (set `self.CurrentAmmo` (`self.MaxAmmo`)))

(event `StartFire`)

(event `StopFire`)

(event `ExecuteAttack`)

(event `PlayAnimMontage`
  (`Character.PlayAnimMontage` (`self.CharacterRef`) (`self.AnimFireMontage`) 1.0 "None"))

(event `ConsumeAmmo`
  (bind _characterref (`self.CharacterRef`))
  (bind _result (`/Engine/EditorBlueprintResources/StandardMacros.DecrementInt` (`self.CurrentAmmo`))
    (:`  `
      (bind _output_get (set `self.CurrentAmmo` _result))
      (if (<= _output_get 0)
        (`self.StopFire`)
        (set `/Game/MyContent/Blueprint/Character/BP_Survivor_Character.CurrentWeaponType` "NewEnumerator0" _characterref)
        (set `/Game/MyContent/Blueprint/Character/BP_Survivor_Character.CurrentWeaponRef` null _characterref)
        (`self.K2_DestroyActor`)))))

(event `self.Sphere.OnComponentBeginOverlap`
  (params (OverlappedComponent :type "PrimitiveComponent Object Reference") (OtherActor :type "Actor Object Reference") (OtherComp :type "PrimitiveComponent Object Reference") (OtherBodyIndex :type Integer) (bFromSweep :type Boolean) (SweepResult :type "HitResult Structure (by ref)"))
  (bind _asbp_survivor_character (cast `/Game/MyContent/Blueprint/Character/BP_Survivor_Character` OtherActor))
  (if (not (`self.IsEquipped`))
    (set `self.IsEquipped` true)
    (`PrimitiveComponent.SetCollisionEnabled` (`self.Sphere`) "NoCollision")
    (`SceneComponent.K2_AttachToComponent` (`self.WeaponMesh`) (`Character.Mesh` _asbp_survivor_character) "WeaponSocketR" "SnapToTarget" "SnapToTarget" "SnapToTarget" true)
    (set `/Game/MyContent/Blueprint/Character/BP_Survivor_Character.CurrentWeaponRef` self _asbp_survivor_character)
    (set `/Game/MyContent/Blueprint/Character/BP_Survivor_Character.CurrentWeaponType` (`self.WeaponType`) _asbp_survivor_character)))

(fn `UserConstructionScript`)