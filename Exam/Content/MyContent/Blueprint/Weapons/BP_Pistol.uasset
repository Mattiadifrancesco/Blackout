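; Pistol weapon Blueprint that fires hitscan shots for the survivor character.
; StartFire checks for remaining ammo, consumes it, plays a montage, then line-traces on the Camera channel from player 0's follow camera along its forward vector, with debug drawing.
; A hit applies base damage and spawns an emitter.
; TargetPoint takes the trace's impact point on both hit and miss, but nothing in this graph reads it.
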(event `self.StartFire`
  (if (not (<= (`self.CurrentAmmo`) 0))
    (`self.ConsumeAmmo`)
    (`self.PlayAnimMontage`)
    (bind _asbp_survivor_character (cast `/Game/MyContent/Blueprint/Character/BP_Survivor_Character` (`GameplayStatics.GetPlayerCharacter` 0)))
    (bind _followcamera (`/Game/MyContent/Blueprint/Character/BP_Survivor_Character.FollowCamera` _asbp_survivor_character))
    (bind _returnvalue (`SceneComponent.K2_GetComponentLocation` _followcamera))
    (bind (_outhit _returnvalue_2) (`KismetSystemLibrary.LineTraceSingle` :`Start` _returnvalue :`End` (+ _returnvalue (* (`SceneComponent.GetForwardVector` _followcamera) 1000000.0)) :`TraceChannel` "TraceTypeQuery2" :`DrawDebugType` "ForDuration"))
    (if _returnvalue_2
      (bind (_bblockinghit _binitialoverlap _time _distance _location _impactpoint _normal _impactnormal _physmat _hitactor) (`GameplayStatics.BreakHitResult` _outhit))
      (set `self.TargetPoint` _impactpoint)
      (`GameplayStatics.ApplyDamage` _hitactor (`self.BaseDMG`))
      (`GameplayStatics.SpawnEmitterAtLocation` null)
      (else
        (set `self.TargetPoint` _impactpoint)))))

(fn `UserConstructionScript`
  (`parent.UserConstructionScript`))