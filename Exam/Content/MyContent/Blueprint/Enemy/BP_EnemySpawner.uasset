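; BP_EnemySpawner is an actor that keeps spawning BP_EnemyBas enemies at its root transform, up to a maximum live count.
; A looping timer started on BeginPlay triggers each spawn attempt, which always spawns regardless of collision while under the cap.
; Each spawned enemy's OnDestroyed event decrements the count and, after a delay, makes another spawn attempt alongside the timer.
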(event `self.ReceiveBeginPlay`
  (`KismetSystemLibrary.K2_SetTimerDelegate` (delegate `SpawnEnemies`) 5.0 true))

(event `SpawnEnemies`
  (if (< (`self.CurrentEnemyCount`) (`self.MaxEnemyCount`))
    (bind _returnvalue (`|SpawnActorFromClass` "/Game/MyContent/Blueprint/Enemy/BP_EnemyBas.BP_EnemyBas_C" (`SceneComponent.K2_GetComponentToWorld` (`self.DefaultSceneRoot`)) "AlwaysSpawn" "MultiplyWithRoot" null null))
    (`/Engine/EditorBlueprintResources/StandardMacros.IncrementInt` (`self.CurrentEnemyCount`)
      (:`  `
        (add `self.OnDestroyed` _returnvalue (delegate `OnEnemyDeath`))))))

(event `OnEnemyDeath` :!signature `self.OnDestroyed`
  (params (DestroyedActor :type "Actor Object Reference"))
  (`/Engine/EditorBlueprintResources/StandardMacros.DecrementInt` (`self.CurrentEnemyCount`)
    (:`  `
      (`KismetSystemLibrary.Delay` 5.0)
      (`self.SpawnEnemies`))))

(fn `UserConstructionScript`)