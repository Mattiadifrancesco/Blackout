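; AI controller for enemies that patrol, then chase and attack the survivor character.
; On possess, it loops moves to random reachable points within a small radius, pausing between them.
; When AI perception senses the survivor, it focuses, speeds up and repeats move-to, AttackPlayer and a short delay.
; Losing the stimulus lowers speed, clears focus and restarts patrol.
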(event `StartPatrol`
  (bind _returnvalue (`self.K2_GetPawn`))
  (`|AIMoveTo` _returnvalue (`NavigationSystemV1.K2_GetRandomReachablePointInRadius` (`self.K2_GetActorLocation` _returnvalue) 300.0 null null) null
    (:`OnSuccess`
      (`KismetSystemLibrary.Delay` 2.0)
      (`self.StartPatrol` :!label _label))))

(event `self.ReceivePossess`
  (params (PossessedPawn :type "Pawn Object Reference"))
  (goto _label))

(event `self.AIPerception.OnTargetPerceptionUpdated`
  (params (Actor :type "Actor Object Reference") (Stimulus :type "AIStimulus Structure"))
  (bind _asbp_survivor_character (cast `/Game/MyContent/Blueprint/Character/BP_Survivor_Character` Actor))
  (if Stimulus_bSuccessfullySensed
    (`self.K2_SetFocus` _asbp_survivor_character)
    (bind _asbp_enemy_bas (cast `/Game/MyContent/Blueprint/Enemy/BP_EnemyBas` (`self.K2_GetPawn`)))
    (bind _charactermovement (`Character.CharacterMovement` _asbp_enemy_bas))
    (set `CharacterMovementComponent.MaxWalkSpeed` 580.0 _charactermovement)
    (`self.StopMovement`)
    (`|AIMoveTo` null (0.0 0.0 0.0) _asbp_survivor_character 85.0 :!label _label_2
      (:`OnSuccess`
        (bind _asbp_enemy_bas_2 (cast `/Game/MyContent/Blueprint/Enemy/BP_EnemyBas` (`self.K2_GetPawn`)))
        (`self.StopMovement`)
        (`/Game/MyContent/Blueprint/Enemy/BP_EnemyBas.AttackPlayer` _asbp_enemy_bas_2)
        (`KismetSystemLibrary.Delay` 0.6)
        (goto _label_2)))
    (else
      (set `CharacterMovementComponent.MaxWalkSpeed` 250.0 _charactermovement)
      (`self.K2_ClearFocus`)
      (`self.StartPatrol`))))

(fn `UserConstructionScript`)