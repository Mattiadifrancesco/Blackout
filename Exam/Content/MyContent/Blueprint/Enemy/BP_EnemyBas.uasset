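; Base enemy character that spawns with a montage, patrols random reachable points, and chases and melees the survivor player.
; PawnSensing sightings speed up the chase, while a retriggerable delay drops it back to slower patrol once sightings stop.
; Attacks are gated by CanAttack and a DoOnce until the montage ends; a separate event deals damage via a jaw-socket sphere trace.
; Damage reduces Health, playing hit reactions or death before destroying the actor.
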(event `self.ReceiveBeginPlay`
  (`self.SetActorHiddenInGame` true)
  (`PrimitiveComponent.SetCollisionResponseToChannel` (`self.Mesh`) "ECC_Camera" "ECR_Ignore")
  (bind _returnvalue (`self.PlayAnimMontage` "/Game/Fab/Zombie_Snapper_-_Hand_Painted_Series/ANIM_EnemySpawn.ANIM_EnemySpawn"))
  (`KismetSystemLibrary.Delay` 0.5)
  (`self.SetActorHiddenInGame` false)
  (`KismetSystemLibrary.Delay` _returnvalue)
  (`self.StartPatrol`))

(event `self.ReceiveAnyDamage`
  (params (Damage :type "Float (single-precision)") (DamageType :type "DamageType Object Reference") (InstigatedBy :type "Controller Object Reference") (DamageCauser :type "Actor Object Reference"))
  (bind _output_get (set `self.Health` (- (`self.Health`) Damage)))
  (if (<= _output_get 0.0)
    (`Controller.UnPossess` (`self.GetController`))
    (bind _returnvalue (`self.PlayAnimMontage` "/Game/Fab/Zombie_Snapper_-_Hand_Painted_Series/ANIM_EnemyDeath.ANIM_EnemyDeath"))
    (`CharacterMovementComponent.SetMovementMode` (`self.CharacterMovement`) "MOVE_None" 0)
    (`PrimitiveComponent.SetCollisionEnabled` (`self.CapsuleComponent`) "NoCollision")
    (`KismetSystemLibrary.Delay` (- _returnvalue 0.3))
    (`self.K2_DestroyActor`)
    (else
      (`self.PlayAnimMontage` "/Game/Fab/Zombie_Snapper_-_Hand_Painted_Series/ANIM_EnemyHit.ANIM_EnemyHit"))))

(event `ExecuteMeleeDamage`
  (bind _returnvalue (`SceneComponent.GetSocketLocation` (`self.Mesh`) "jaw"))
  (bind (_outhit _returnvalue_2) (`KismetSystemLibrary.SphereTraceSingle` _returnvalue _returnvalue 100.0 "TraceTypeQuery2" false (`|MakeArray` self :!type "Actor Object Reference")))
  (if _returnvalue_2
    (bind _asbp_survivor_character (cast `/Game/MyContent/Blueprint/Character/BP_Survivor_Character` (`.HitActor` (`GameplayStatics.BreakHitResult` _outhit))))
    (`GameplayStatics.ApplyDamage` _asbp_survivor_character 18.0)))

(event `StartPatrol`
  (`|AIMoveTo` self (`NavigationSystemV1.K2_GetRandomReachablePointInRadius` (`self.K2_GetActorLocation`) 1000.0 null null) null
    (:`OnSuccess`
      (`KismetSystemLibrary.Delay` 2.0)
      (`self.StartPatrol`))))

(event `self.PawnSensing.OnSeePawn`
  (params (Pawn :type "Pawn Object Reference"))
  (bind _charactermovement (`self.CharacterMovement`))
  (set `self.CanAttack` true)
  (`|ExecutionSequence`
    (:`then_0`
      (set `CharacterMovementComponent.MaxWalkSpeed` 580.0 _charactermovement)
      (`|AIMoveTo` self (0.0 0.0 0.0) (`GameplayStatics.GetPlayerCharacter` 0) 100.0
        (:`OnSuccess`
          (if (`self.CanAttack`)
            (set `self.CanAttack` false)
            (`self.AttackPlayer`)))))
    (:`then_1`
      (`KismetSystemLibrary.RetriggerableDelay` 1.0)
      (`self.StartPatrol`)
      (set `CharacterMovementComponent.MaxWalkSpeed` 300.0 _charactermovement))))

(event `AttackPlayer`
  (bind _asbp_survivor_character (cast `/Game/MyContent/Blueprint/Character/BP_Survivor_Character` (`GameplayStatics.GetPlayerCharacter` 0)))
  (if (not (`/Game/MyContent/Blueprint/Character/BP_Survivor_Character.IsDead` _asbp_survivor_character))
    (`/Engine/EditorBlueprintResources/StandardMacros.DoOnce` false :!label _label
      (:`Completed`
        (bind _returnvalue (`self.PlayAnimMontage` "/Game/Fab/Zombie_Snapper_-_Hand_Painted_Series/ANIM_EnemyAttack.ANIM_EnemyAttack"))
        (`KismetSystemLibrary.Delay` _returnvalue)
        (set `self.CanAttack` true)
        (goto _label :!via `Reset`)))))

(fn `UserConstructionScript`)