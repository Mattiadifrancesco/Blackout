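; BP_WeaponSpawner is a weapon spawn point that keeps a random weapon available in the level.
; On BeginPlay it picks a random class from WeaponsToSpawn and spawns it at SpawnPoint, always spawning regardless of collision.
; It binds to the spawned weapon's OnDestroyed event, treating destruction as a pickup, then waits CooldownSpawn before spawning another random weapon.
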(event `SpawnRandomWeapon`
  (bind _returnvalue (`|SpawnActorFromClass` (`KismetArrayLibrary.Array_Random` (`self.WeaponsToSpawn`)) (`SceneComponent.K2_GetComponentToWorld` (`self.SpawnPoint`)) "AlwaysSpawn" "MultiplyWithRoot" null null))
  (bind _output_get (set `self.CurrentSpawnedWeapon` _returnvalue))
  (add `self.OnDestroyed` _output_get (delegate `WeaponPickup`)))

(event `WeaponPickup` :!signature `self.OnDestroyed`
  (params (DestroyedActor :type "Actor Object Reference"))
  (`KismetSystemLibrary.Delay` (`KismetMathLibrary.Conv_IntToDouble` (`self.CooldownSpawn`)))
  (`self.SpawnRandomWeapon`))

(event `self.ReceiveBeginPlay`
  (`self.SpawnRandomWeapon`))

(fn `UserConstructionScript`)